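; BP_IncreaseVelocity is a power-down obstacle that triples the player pawn's Speed on contact.
; Its mesh overlap event passes a DoOnce, then compares the other actor to Pawn before multiplying Speed and calling OnDestroy.
; The DoOnce precedes that check, so a first overlap by any other actor uses up the trigger.
; The speed change has no timer or revert here.
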(event OnComponentBeginOverlap(Mesh)
  (params (OverlappedComponent :type Primitive%20Component%20Object%20Reference) (OtherActor :type Actor%20Object%20Reference) (OtherComp :type Primitive%20Component%20Object%20Reference) (OtherBodyIndex :type Integer) (bFromSweep :type Boolean) (SweepResult :type Hit%20Result%20Structure%20%28by%20ref%29))
  (bind _pawn (Variables|Default|GetPawn))
  (Utilities|FlowControl|DoOnce false
    (:Completed
      (if (== OtherActor _pawn)
        (Variables|/Game/Blueprints/BP_PlayerPawn.BP_PlayerPawn_C|SetSpeed _pawn (* (Variables|/Game/Blueprints/BP_PlayerPawn.BP_PlayerPawn_C|GetSpeed _pawn) 3.0))
        (CallFunction|OnDestroy)))))

(event EventBeginPlay
  (|CallParentFunction))

(event Collision|EventActorBeginOverlap
  (params (OtherActor :type Actor%20Object%20Reference)))

(event EventTick
  (params (DeltaSeconds :type Float%20%28single-precision%29)))

(fn ConstructionScript
  (|CallParentFunction))