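; BP_Shifter is an obstacle actor in the PowerDown folder that shifts its location through a timeline.
; Tick calls PlayFromStart on TimelineShigter every frame, so the timeline keeps restarting.
; Each timeline update adds the Movement vector to the current actor location as a relative offset, without sweep.
; The Finished branch subtracts Movement once through a single-pass loop, then calls Play again.
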(event EventBeginPlay
  (|CallParentFunction))

(event Collision|EventActorBeginOverlap
  (params (OtherActor :type Actor%20Object%20Reference)))

(event EventTick
  (params (DeltaSeconds :type Float%20%28single-precision%29))
  (bind _returnvalue (Transformation|GetActorLocation))
  (bind _movement_ (Timeline|Timeline%20Shigter PlayFromStart)
    (:Update
      (Transformation|SetActorLocation (+ _returnvalue _movement_) false false))
    (:Finished
      (for _index (range 1 1)
        (Transformation|SetActorLocation (- _returnvalue _movement_) false false))
      (Timeline|Timeline%20Shigter Play))))

(fn ConstructionScript
  (|CallParentFunction))