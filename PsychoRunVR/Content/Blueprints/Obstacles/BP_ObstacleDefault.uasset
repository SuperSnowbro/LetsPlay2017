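; BP_ObstacleDefault is an obstacle actor that acts as either a hazard or a powerup, depending on its ObstacleType.
; It caches the first BP_PlayerPawn at BeginPlay and reacts only when that pawn overlaps its Trigger.
; On contact it destroys itself through OnDestroy, which prints a debug message, then plays the type's sound at world origin and calls the pawn's bad or good hit feedback.
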(event OnComponentBeginOverlap(Trigger)
  (params (OverlappedComponent :type Primitive%20Component%20Object%20Reference) (OtherActor :type Actor%20Object%20Reference) (OtherComp :type Primitive%20Component%20Object%20Reference) (OtherBodyIndex :type Integer) (bFromSweep :type Boolean) (SweepResult :type Hit%20Result%20Structure%20%28by%20ref%29))
  (bind _pawn (Variables|Default|GetPawn))
  (if (== OtherActor (Variables|Default|GetPawn))
    (CallFunction|OnDestroy)
    (switch Utilities|FlowControl|Switch|SwitchonE_ObstacleType (Variables|Default|GetObstacle%20Type)
      (:NewEnumerator1
        (Audio|PlaySoundatLocation "/Game/Media/Sound/Hit.Hit" "0, 0, 0")
        (Default|BadObstacleHitFeedback _pawn))
      (:NewEnumerator2
        (Audio|PlaySoundatLocation "/Game/Media/Sound/Power_Up.Power_Up" "0, 0, 0")
        (Default|GoodObstacleHitFeedback _pawn)))))

(event Custom|OnDestroy
  (Actor|DestroyActor)
  (Development|PrintString "Ostacolo Colpito"))

(event EventBeginPlay
  (bind _outactors (Actor|GetAllActorsOfClass "/Game/Blueprints/BP_PlayerPawn.BP_PlayerPawn_C"))
  (Variables|Default|SetPawn (Utilities|Array|Get(acopy) _outactors)))

(fn ConstructionScript)