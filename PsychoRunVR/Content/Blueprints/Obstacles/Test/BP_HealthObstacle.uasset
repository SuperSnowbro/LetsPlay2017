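; BP_HealthObstacle is a test obstacle that acts as a health pickup, granting the player an extra life on contact.
; Its only active logic is the overlap event, which checks the other actor against BP_PlayerPawn, increments Lives and prints "+1".
; It does not destroy or disable itself, so each new overlap can grant another life.
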(event EventBeginPlay
  (|CallParentFunction))

(event Collision|EventActorBeginOverlap
  (params (OtherActor :type Actor%20Object%20Reference))
  (bind _player (Variables|Default|Getplayer))
  (if (== OtherActor "/Game/Blueprints/BP_PlayerPawn.BP_PlayerPawn")
    (Variables|/Game/Blueprints/BP_PlayerPawn.BP_PlayerPawn_C|SetLives _player (+ (Variables|/Game/Blueprints/BP_PlayerPawn.BP_PlayerPawn_C|GetLives _player) 1))
    (Development|PrintString "+1")))

(event EventTick
  (params (DeltaSeconds :type Float%20%28single-precision%29)))

(fn ConstructionScript
  (|CallParentFunction))