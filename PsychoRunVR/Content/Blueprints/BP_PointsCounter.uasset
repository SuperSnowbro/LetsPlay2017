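; BP_PointsCounter keeps a running Points score that grows over time and changes with obstacle events.
; Tick prints the score and calls a delay-based graph, which relies on the pending Delay ignoring re-triggers to add roughly one point per second.
; UpdatePointsCounter adds or subtracts a point depending on which of two obstacle types it receives.
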(event EventUpdatePointsCounter
  (params (Obstacle%20Type :type E_ObstacleType%20Enum :default "NewEnumerator0"))
  (if (Utilities|Enum|Equal(Enum) Obstacle%20Type "NewEnumerator1")
    (Variables|Default|SetPoints (- (Variables|Default|GetPoints) 1))
    (elif (Utilities|Enum|Equal(Enum) Obstacle%20Type "NewEnumerator2")
      (Variables|Default|SetPoints (+ (Variables|Default|GetPoints) 1)))))

(event EventTick
  (params (DeltaSeconds :type Float%20%28single-precision%29))
  (Development|PrintString (Utilities|String|ToString(Integer) (Variables|Default|GetPoints)))
  (|UpdatePoints*Seconds))

(fn ConstructionScript)