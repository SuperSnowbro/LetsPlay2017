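; BP_TestPawn is a test VR pawn that moves a Cube forward at constant Speed and rolls it with the player's head movement.
; Each tick it advances the Cube along relative X, integrates headset sideways position into roll, and applies headset rotation to the Camera.
; Despite the function name, spline lookups are unused.
; H resets headset position; the Lifes check (ControlloVita) has empty branches.
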(event EventBeginPlay)

(event Collision|EventActorBeginOverlap
  (params (OtherActor :type Actor%20Object%20Reference)))

(event EventTick
  (params (DeltaSeconds :type Float%20%28single-precision%29))
  (CallFunction|IncreaseDistance)
  (CallFunction|UpdateTransformAlongSpline)
  (Variables|Default|SetCurrentRotation (+ (Variables|Default|GetCurrentRotation) (* (* (.y (.DevicePosition (Class|HeadMountedDisplayFunctionLibrary|GetOrientationandPosition))) -1.0) (Utilities|Time|GetWorldDeltaSeconds) (Variables|Default|GetTurnRate))))
  (Transformation|SetRelativeRotation (Variables|Default|GetCamera) (.DeviceRotation (Class|HeadMountedDisplayFunctionLibrary|GetOrientationandPosition)) false true)
  (|ControlloVita))

(event Input|KeyboardEvents|H
  (params (Key :type Key%20Structure :default "AnyKey"))
  (:Pressed
    (Class|HeadMountedDisplayFunctionLibrary|ResetOrientationandPosition 0.0 "Position")))

(fn ConstructionScript)

(fn IncreaseDistance
  (Variables|Default|SetCurrentDistance (+ (* (Utilities|Time|GetWorldDeltaSeconds) (Variables|Default|GetSpeed)) (Variables|Default|GetCurrentDistance))))

(fn UpdateTransformAlongSpline
  (Transformation|SetRelativeLocation (Variables|Default|GetCube) (Math|Vector|MakeVector (Variables|Default|GetCurrentDistance) 0.0 0.0) false true)
  (Transformation|SetRelativeRotation (Variables|Default|GetCube) (Math|Rotator|MakeRotator (Variables|Default|GetCurrentRotation) 0.0 0.0) false false))