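; BP_ObstaclesManager spawns random obstacles along the spline system while its spawn cycle is switched on.
; Tick raises a time counter scaled by SpawnSpeed; crossing zero subtracts a random delay and spawns a random class from ObstaclesList.
; Each obstacle takes location, pitch and yaw from the spline at ObstacleSpawnDistance.
; Its roll follows the player pawn's current rotation plus a random offset within ObstacleRotationDelta.
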(event Custom|OnSpawnObstacle
  (params (Selected%20Obstacle :type Integer))
  (CallFunction|SpawnObstacleintheLevel Selected%20Obstacle))

(event Custom|BreakSpawnCycle
  (Variables|Default|SetisSpawning false))

(event Custom|BeginSpawnCycle
  (Variables|Default|SetisSpawning true)
  (CallFunction|ResetSpawnTimeCounter))

(event EventBeginPlay)

(event EventTick
  (params (DeltaSeconds :type Float%20%28single-precision%29))
  (if (Variables|Default|GetisSpawning)
    (CallFunction|AttemptIncrementSpawnTimeCounter)
    (if (> (Variables|Default|GetSpawnTimeCounter) 0.0)
      (CallFunction|ResetSpawnTimeCounter)
      (CallFunction|OnSpawnObstacle (Math|Random|RandomInteger (Utilities|Array|Length (Variables|Default|GetObstaclesList)))))))

(fn ConstructionScript)

(fn SpawnObstacleintheLevel
  (params (Selected :type Integer))
  (bind _splinesystem (Variables|Default|GetSplineSystem))
  (bind _obstaclerotationdelta (Variables|Tuning|GetObstacleRotationDelta))
  (bind _obstaclespawndistance (Variables|Tuning|GetObstacleSpawnDistance))
  (bind (_location _rotation_y _rotation_z) (Default|GetObstacleLocationandRotation _splinesystem _obstaclespawndistance))
  (bind _returnvalue (Game|SpawnActorfromClass (Utilities|Array|Get(acopy) (Variables|Default|GetObstaclesList) Selected) (Math|Transform|MakeTransform _location (Math|Rotator|MakeRotator (+ (Variables|/Game/Blueprints/BP_PlayerPawn.BP_PlayerPawn_C|GetCurrentRotation (Variables|Default|GetPlayerPawn)) (Math|Random|RandomFloatinRange (* _obstaclerotationdelta -1.0) _obstaclerotationdelta)) _rotation_y _rotation_z)) "Undefined" 0 0))
  (return _returnvalue))

(fn AttemptIncrementSpawnTimeCounter
  (Variables|Default|SetSpawnTimeCounter (+ (Variables|Default|GetSpawnTimeCounter) (* (Utilities|Time|GetWorldDeltaSeconds) (Variables|Tuning|GetSpawnSpeed))))
  (return))

(fn ResetSpawnTimeCounter
  (Variables|Default|SetSpawnTimeCounter (- (Variables|Default|GetSpawnTimeCounter) (Math|Random|RandomFloatinRange (Variables|Tuning|GetMinSpawnDelay) (Variables|Tuning|GetMaxSpawnDelay)))))