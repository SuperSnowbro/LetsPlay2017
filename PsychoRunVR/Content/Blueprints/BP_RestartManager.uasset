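; BP_RestartManager is an actor that returns the test pawn to the manager's own location, acting as a simple restart.
; BeginPlay caches the first BP_TestPawn found, waits through a fixed delay, then sets an Invoke flag.
; Tick calls RestartLevel through a DoOnce that resets immediately, so the pawn is repositioned every frame while Invoke stays true.
; RestartLevel only moves the pawn, without reloading the level.
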(event Custom|Restart%20Level
  (params (Player :type Actor%20Object%20Reference))
  (Transformation|SetActorLocation Player (Transformation|GetActorLocation self) false false))

(event EventBeginPlay
  (bind _outactors (Actor|GetAllActorsOfClass "/Game/Blueprints/BP_TestPawn.BP_TestPawn_C"))
  (Variables|Default|SetMyPawn (Utilities|Array|Get(acopy) _outactors))
  (Utilities|FlowControl|Delay 3e+01)
  (Variables|Default|SetInvoke? true))

(event EventTick
  (params (DeltaSeconds :type Float%20%28single-precision%29))
  (if (Variables|Default|GetInvoke?)
    (Utilities|FlowControl|DoOnce false :!label _label
      (:Completed
        (CallFunction|RestartLevel (Variables|Default|GetMyPawn))
        (goto _label Reset)))))

(fn ConstructionScript)