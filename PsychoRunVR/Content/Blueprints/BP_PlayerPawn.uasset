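; VR player pawn for an obstacle game, looping along a spline at CurrentSpeed and rolling around it from the headset's lateral position through a remap curve.
; Space recenters the headset and starts the game once via GameManager.
; BeginGame ramps up speed with a timeline, then starts obstacle spawning.
; Bad hits trigger a camera fade and timed slowdown; good-hit feedback and the lives check (Controllo Vita) are empty stubs.
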(event Custom|BeginGame
  (bind _alpha (Timeline|InterpSpeed Play)
    (:Update
      (Variables|Default|SetCurrentSpeed (Math|Float|Lerp 0.0 (Variables|Tuning|GetSpeed) _alpha)))
    (:Finished
      (Default|BeginSpawnCycle (Variables|Default|GetObstacleManager)))))

(event Custom|BadObstacleHitFeedback
  (CameraFades|StartCameraFade (Game|GetPlayerCameraManager 0) (Variables|FeedbackTuning|GetBadObstacleHitFadeAlpha) 0.0 (Variables|FeedbackTuning|GetBadObstacleHitDuration) (Variables|FeedbackTuning|GetBadObstacleHitFeedbackColor) false true)
  (Components|Timeline|SetPlayRate (Variables|Default|GetHitSlowDown) (/ 1.0 (Variables|FeedbackTuning|GetBadObstacleHitDuration)))
  (bind _alpha (Timeline|HitSlowDown PlayFromStart)
    (:Update
      (Variables|Default|SetCurrentSpeed (* (Variables|Tuning|GetSpeed) (Math|Float|Lerp (Variables|FeedbackTuning|GetHitSlowDownMultiplier) 1.0 _alpha))))))

(event Custom|GoodObstacleHitFeedback)

(event EventTick
  (params (DeltaSeconds :type Float%20%28single-precision%29))
  (CallFunction|IncreaseDistance)
  (CallFunction|UpdateTransform)
  (CallFunction|PlayerInput)
  (|ControlloVita))

(event Input|KeyboardEvents|SpaceBar
  (params (Key :type Key%20Structure :default "AnyKey"))
  (:Pressed
    (Class|HeadMountedDisplayFunctionLibrary|ResetOrientationandPosition 0.0 "Position")
    (Utilities|FlowControl|DoOnce false
      (:Completed
        (Default|StartGame (Variables|Default|GetGameManager))))))

(fn ConstructionScript)

(fn IncreaseDistance
  (Variables|Default|SetCurrentDistance (+ (* (Utilities|Time|GetWorldDeltaSeconds) (Variables|Default|GetCurrentSpeed)) (Variables|Default|GetCurrentDistance)))
  (if (> (Variables|Default|GetCurrentDistance) (Spline|GetSplineLength (Variables|/Game/Blueprints/BP_SPlineSystemSnow.BP_SPlineSystemSnow_C|GetSpline (Variables|Default|GetSplineSystem))))
    (Variables|Default|SetCurrentDistance (- (Variables|Default|GetCurrentDistance) (Spline|GetSplineLength (Variables|/Game/Blueprints/BP_SPlineSystemSnow.BP_SPlineSystemSnow_C|GetSpline (Variables|Default|GetSplineSystem)))))))

(fn UpdateTransform
  (bind _currentdistance (Variables|Default|GetCurrentDistance))
  (bind _splinesystem (Variables|Default|GetSplineSystem))
  (bind _spline (Variables|/Game/Blueprints/BP_SPlineSystemSnow.BP_SPlineSystemSnow_C|GetSpline _splinesystem))
  (bind _returnvalue (Spline|GetRotationatDistanceAlongSpline _spline _currentdistance "World"))
  (Transformation|SetWorldLocationAndRotation (Variables|Default|GetCenter) (Spline|GetLocationatDistanceAlongSpline _spline (Variables|Default|GetCurrentDistance) "World") (Math|Rotator|MakeRotator (Variables|Default|GetCurrentRotation) (.pitch _returnvalue) (.yaw _returnvalue)) false true))

(fn PlayerInput
  (bind _deviceposition (Class|HeadMountedDisplayFunctionLibrary|GetOrientationandPosition))
  (bind _inputsensitivity (LocalVariables|GetInputSensitivity))
  (bind _inputremapcurve (Variables|Default|GetInputRemapCurve))
  (bind _isoutside (Variables|Default|GetIsOutside))
  (bind _returnvalue (* (.y _deviceposition) -1.0))
  (bind _returnvalue_2 (Math|Float|SelectFloat (.y _deviceposition) _returnvalue _isoutside))
  (bind _returnvalue_3 (/ _returnvalue_2 _inputsensitivity))
  (bind _returnvalue_4 (Math|Float|Clamp(Float) _returnvalue_3 -1.0))
  (bind _returnvalue_5 (Math|Float|Absolute(Float) _returnvalue_4))
  (bind _returnvalue_6 (Math|Curves|GetFloatValue _inputremapcurve _returnvalue_5))
  (Variables|Default|SetCurrentRotation (+ (Variables|Default|GetCurrentRotation) (* (Math|Float|SelectFloat _returnvalue_6 (* _returnvalue_6 -1.0) (> _returnvalue_4 0.0)) (Utilities|Time|GetWorldDeltaSeconds) (Variables|Tuning|GetTurnRate))))
  (Transformation|SetRelativeRotation (Variables|Default|GetCamera) (.DeviceRotation (Class|HeadMountedDisplayFunctionLibrary|GetOrientationandPosition)) false true)
  (return))