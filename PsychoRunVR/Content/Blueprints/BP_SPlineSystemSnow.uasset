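; Snow spline track actor that builds a mesh path and supplies placement transforms for obstacles ahead of the player.
; The construction script adds a spline mesh component between each pair of spline points, matching their locations and tangents.
; GetObstacleLocationAndRotation offsets the player's current distance by ObstacleDistance, wrapping once past the spline's end.
; It returns that point's world location, pitch and yaw, omitting roll.
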(fn ConstructionScript
  (Utilities|FlowControl|Sequence
    (:then_0
      (for _index (range 0 (- (Spline|GetNumberOfSplinePoints (Variables|Default|GetSpline)) 2))
        (bind _returnvalue (AddComponent|AddSplineMeshComponent true))
        (Transformation|AttachComponentToComponent _returnvalue (Variables|Default|GetSpline) "None" "KeepRelative" "KeepRelative" "KeepRelative" true)
        (SplineMesh|SetStartandEnd _returnvalue (.Location (Spline|GetLocationandTangentatSplinePoint (Variables|Default|GetSpline) _index "Local")) (.Tangent (Spline|GetLocationandTangentatSplinePoint (Variables|Default|GetSpline) _index "Local")) (.Location (Spline|GetLocationandTangentatSplinePoint (Variables|Default|GetSpline) (+ _index 1) "Local")) (.Tangent (Spline|GetLocationandTangentatSplinePoint (Variables|Default|GetSpline) (+ _index 1) "Local")) true :!class /Script/Engine.SplineMeshComponent)
        (Components|StaticMesh|SetStaticMesh _returnvalue (Variables|Default|GetMesh))))))

(fn GetObstacleLocationandRotation
  (bind _player (Variables|Default|GetPlayer))
  (bind _obstacledistance (Variables|Default|GetObstacleDistance))
  (bind _currentdistance (Variables|/Game/Blueprints/BP_PlayerPawn.BP_PlayerPawn_C|GetCurrentDistance _player))
  (bind _returnvalue (+ _currentdistance _obstacledistance))
  (LocalVariables|SetObstacleDistanceAlongSpline _returnvalue)
  (if (> _returnvalue (Spline|GetSplineLength (Variables|Default|GetSpline)))
    (LocalVariables|SetObstacleDistanceAlongSpline (- (LocalVariables|GetObstacleDistanceAlongSpline) (Spline|GetSplineLength (Variables|Default|GetSpline)))))
  (return (Spline|GetLocationatDistanceAlongSpline (Variables|Default|GetSpline) (LocalVariables|GetObstacleDistanceAlongSpline) "World") (.pitch (Spline|GetRotationatDistanceAlongSpline (Variables|Default|GetSpline) (LocalVariables|GetObstacleDistanceAlongSpline) "World")) (.yaw (Spline|GetRotationatDistanceAlongSpline (Variables|Default|GetSpline) (LocalVariables|GetObstacleDistanceAlongSpline) "World"))))