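; Test actor for a snow fractured mesh that breaks itself one second after BeginPlay.
; It applies a dynamic obstacle-explosion material to both mesh slots, then shatters the mesh with a massive damage hit and impulse.
; A FractureMesh timeline drives the material's AnimationTime parameter, and the actor destroys itself when the timeline finishes.
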(event Custom|BreakMesh
  (bind _sm_testfracturedmesh (Variables|Default|GetSM_TestFracturedMesh))
  ;[1 1 1] spacca la mesh!
  (Game|Damage|ApplyDamage _sm_testfracturedmesh 99999.0 (Transformation|GetWorldLocation _sm_testfracturedmesh) (Math|Vector|MakeVector 1.0 0.0 0.0) 4444.0))

(event EventBeginPlay
  (Utilities|FlowControl|Delay 1.0)
  (bind _returnvalue (Rendering|Material|CreateDynamicMaterialInstance "/Game/Materials/MaterialInstances/MI_ObstacleExplosion.MI_ObstacleExplosion" :!class /Script/Engine.KismetMaterialLibrary))
  (Variables|Default|SetDynamic%20Material%20Instance _returnvalue)
  (Rendering|Material|SetMaterial (Variables|Default|GetSM_TestFracturedMesh) 0 (Variables|Default|GetDynamic%20Material%20Instance))
  (Rendering|Material|SetMaterial (Variables|Default|GetSM_TestFracturedMesh) 1 (Variables|Default|GetDynamic%20Material%20Instance))
  (CallFunction|BreakMesh)
  (bind _animationtime (Timeline|FractureMesh Play)
    (:Update
      (Rendering|Material|SetScalarParameterValue (Variables|Default|GetDynamic%20Material%20Instance) "AnimationTime" _animationtime :!class /Script/Engine.MaterialInstanceDynamic))
    (:Finished
      (Actor|DestroyActor))))

(fn ConstructionScript)